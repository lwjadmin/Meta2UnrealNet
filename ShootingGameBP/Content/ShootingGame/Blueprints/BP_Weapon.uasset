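; Multiplayer gun actor that takes its mesh, sound, effect, montages and reload ammo from WeaponData, and attaches to or physically drops from a character.
; Trigger and reload play montages, while notify events fire shots and refill ammo.
; Shots show effects immediately, then the local player requests a server shot that spends ammo, line-traces from the camera and damages hit Characters.
; Ammo's RepNotify updates the owning player's HUD.
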(event Custom|ReqShoot
  (params (StartPoint :type Vector) (ForwardVector :type Vector))
  ;[1 0 0] RUN ON SERVER(후보고)
  (bind _iscanshoot (CallFunction|UseAmmo))
  (if _iscanshoot
    (CallFunction|ProcessServerShoot StartPoint ForwardVector)))

(event EventBeginPlay
  (Audio|Components|Audio|SetSound (Variables|Default|GetAudio) (.shootsound (Variables|Default|GetWeaponData)))
  (Components|StaticMesh|SetStaticMesh (Variables|Default|GetStaticMesh) (.staticmesh (Variables|Default|GetWeaponData))))

(event EventReloadEvent
  (Animation|PlayAnimMontage (Variables|Default|GetOwnCharacter) (.reloadmontage (Variables|Default|GetWeaponData)) 1.0 "None"))

(event EventNotifyReload
  (CallFunction|DoReload))

(event EventTriggerEvent
  (params (IsPressed :type Boolean))
  (if IsPressed
    (Animation|PlayAnimMontage (Variables|Default|GetOwnCharacter) (.shootmontage (Variables|Default|GetWeaponData)) 1.0 "None")))

(event EventNotifyShoot
  (bind _returnvalue (Game|GetPlayerCameraManager 0))
  ;[0 0 1] CLIENT(선처리)
  (bind _iscanuse (CallFunction|IsCanUse))
  (if _iscanuse
    (CallFunction|ShowShootingEffect)
    ;;[1 1 1] 데미지 요청 처리
    (if (== (Variables|Default|GetOwnCharacter) (Game|GetPlayerCharacter 0))
      (CallFunction|ReqShoot (Transformation|GetActorLocation _returnvalue) (Transformation|GetActorForwardVector _returnvalue)))))

(fn ConstructionScript)

(fn UseAmmo
  (LocalVariables|SetCanUsed (> (Variables|Default|GetAmmo) 0))
  (Variables|Default|SetAmmo (Math|Integer|Clamp(Integer) (- (Variables|Default|GetAmmo) 1) 0 30))
  (return (LocalVariables|GetCanUsed)))

(fn OnRepAmmo
  (CallFunction|UpdateAmmoUI (Variables|Default|GetAmmo)))

(fn UpdateAmmoUI
  (params (Ammo :type Integer))
  (Utilities|IsValid (Variables|Default|GetOwnCharacter)
    (:Is%20Valid
      (if (== (Pawn|GetController (Variables|Default|GetOwnCharacter)) (Game|GetPlayerController 0))
        (bind _asshooting_hud (Utilities|Casting|CastToShootingHud (HUD|GetHUD (Game|GetPlayerController 0)))
          (:then
            (Default|SetAmmo (Variables|/Game/ShootingGame/GameMode/ShootingHud.ShootingHud_C|GetHudWidget _asshooting_hud) Ammo))
          (:CastFailed
            (Development|PrintString "ERR3")))
        (else
          (Development|PrintString "ERR2"))))
    (:Is%20Not%20Valid
      (Development|PrintString "ERR1"))))

(fn ShowShootingEffect
  (bind _staticmesh (Variables|Default|GetStaticMesh))
  (bind _returnvalue (Transformation|GetSocketTransform _staticmesh "Muzzle" "RTS_World"))
  (Effects|SpawnEmitteratLocation (.shooteffect (Variables|Default|GetWeaponData)) (.location _returnvalue) (.rotation _returnvalue) "0.300000,0.300000,0.300000" true "AutoRelease")
  (Audio|Components|Audio|Play (Variables|Default|GetAudio) 0.0))

(fn ProcessServerShoot
  (params (StartPoint :type Vector) (ForwardVector :type Vector))
  (bind _outhit (Collision|LineTraceForObjects (+ StartPoint (* ForwardVector 3.5e+02)) (+ StartPoint (* ForwardVector (Variables|Default|GetDistance))) (Utilities|Array|MakeArray "ObjectTypeQuery3" "ObjectTypeQuery1" "ObjectTypeQuery2" "ObjectTypeQuery4" "ObjectTypeQuery5" "ObjectTypeQuery6") false (Utilities|Array|MakeArray (Variables|Default|GetOwnCharacter)) "Persistent"))
  (Development|PrintString (Utilities|String|Append "HitActor - " (Utilities|GetDisplayName (.HitActor (Collision|BreakHitResult _outhit)))) true true "(R=0.000000,G=0.660000,B=1.000000,A=1.000000)" 6e+01)
  (bind _ascharacter (Utilities|Casting|CastToCharacter (.HitActor (Collision|BreakHitResult _outhit))))
  (Game|Damage|ApplyDamage _ascharacter 1e+01 (Pawn|GetController (Variables|Default|GetOwnCharacter)) self))

(fn DoReload
  (Variables|Default|SetAmmo (.ammo (Variables|Default|GetWeaponData))))

(fn AttachWeapon
  (params (Character :type Character%20Object%20Reference))
  (Variables|Default|SetOwnCharacter Character)
  (Physics|SetSimulatePhysics (Variables|Default|GetStaticMesh) false)
  (Collision|SetCollisionEnabled (Variables|Default|GetStaticMesh) "NoCollision")
  ;[1 1 1] CharacterMesh에 붙이기 위해 Snap/Snap/KeepWorld!
  (Transformation|AttachComponentToComponent (Variables|/Script/Engine.Character|GetMesh (Variables|Default|GetOwnCharacter)) "weapon" "SnapToTarget" "SnapToTarget" "KeepWorld" true)
  (CallFunction|UpdateAmmoUI (Variables|Default|GetAmmo))
  (return true))

(fn DetachWeapon
  (CallFunction|UpdateAmmoUI)
  (Variables|Default|SetOwnCharacter 0)
  (Transformation|DetachFromComponent (Variables|Default|GetStaticMesh) "KeepWorld" "KeepWorld" "KeepWorld" true)
  (Collision|SetCollisionEnabled (Variables|Default|GetStaticMesh) "QueryAndPhysics")
  (Physics|SetSimulatePhysics (Variables|Default|GetStaticMesh) true)
  (return true))

(fn IsCanUse
  (return (> (Variables|Default|GetAmmo) 0)))