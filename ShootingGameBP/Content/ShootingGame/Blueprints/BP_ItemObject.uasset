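; BP_ItemObject is a world item pickup in the shooting game, identified by a row name in the DT_Item data table.
; On BeginPlay it looks up that row and applies its static mesh to the component when valid.
; When an actor overlaps the mesh, it passes the row name to that actor's BP_InvenComponent.
; It destroys itself only if the item is accepted, otherwise printing an inventory-full message.
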(event OnComponentBeginOverlap(StaticMesh)
  (params (OverlappedComponent :type Primitive%20Component%20Object%20Reference) (OtherActor :type Actor%20Object%20Reference) (OtherComp :type Primitive%20Component%20Object%20Reference) (OtherBodyIndex :type Integer) (bFromSweep :type Boolean) (SweepResult :type Hit%20Result%20Structure%20%28by%20ref%29))
  ;[1 1 1] 먹었는데, 인벤에 빈칸이 없으면 Destroy되지 않음!!!
  (bind _success (Default|GetItem (Actor|GetComponentbyClass OtherActor "/Game/ShootingGame/Data/BP_InvenComponent.BP_InvenComponent_C") (Variables|Default|GetItemRowName)))
  (if _success
    (Actor|DestroyActor)
    (else
      (Development|PrintString "인벤토리가 가득찼습니다!!!"))))

(event EventBeginPlay
  (bind _returnvalue (Utilities|GetDataTableRow "/Game/ShootingGame/Data/DT_Item.DT_Item" (Variables|Default|GetItemRowName))
    (:then
      (bind _output_get (Variables|Default|SetItem _returnvalue))
      (Utilities|IsValid (.StaticMesh (Utilities|Struct|BreakST_Item _output_get))
        (:Is%20Valid
          (Components|StaticMesh|SetStaticMesh (Variables|Default|GetStaticMesh) (.StaticMesh (Utilities|Struct|BreakST_Item _output_get))))))))

(fn ConstructionScript)