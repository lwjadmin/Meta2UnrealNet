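; Burst weapon Blueprint for the shooting game that repeats its shot animation for as long as the trigger is held.
; TriggerEvent calls BurstShooting on press and starts a fast looping timer by function name, which it clears on release.
; Each BurstShooting call checks IsCanUse, then plays the ShootMontage from WeaponData on the owning character; the graph itself contains no projectile or damage logic.
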(event EventBeginPlay
  (|CallParentFunction) ; This node is disabled and will not be called.\nDrag off pins to build functionality.
)

(event Collision|EventActorBeginOverlap
  (params (OtherActor :type Actor%20Object%20Reference)))

(event EventTriggerEvent
  (params (IsPressed :type Boolean))
  (if IsPressed
    (Utilities|Time|SetTimerbyFunctionName 0 "BurstShooting" 0.1 true)
    (CallFunction|BurstShooting)
    (else
      (Utilities|Time|ClearTimerbyFunctionName 0 "BurstShooting"))))

(fn ConstructionScript
  (|CallParentFunction))

(fn BurstShooting
  (bind _iscanuse (CallFunction|IsCanUse))
  (if _iscanuse
    (Animation|PlayAnimMontage (Variables|Default|GetOwnCharacter) (.shootmontage (Variables|Default|GetWeaponData)) 1.0 "None")))